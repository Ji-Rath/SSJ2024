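; BP_MovingFloor is an environment tool actor that emits a moving stream of BP_TrailSpline actors to act as a moving floor.
; A looping timer spawns a piece at the actor's location every second, gives it a short lifespan and adds it to LevelsLoaded.
; Tick offsets each valid piece by Velocity scaled by delta time, without sweeping.
; Expired entries are skipped but never removed from the array.
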(event Custom|CustomEvent
  (bind _returnvalue (Game|SpawnActorfromClass "/Game/Environment/Tools/BP_TrailSpline.BP_TrailSpline_C" (Math|Conversions|ToTransform(Vector) (Transformation|GetActorLocation)) "AlwaysSpawn" "MultiplyWithRoot" 0 0))
  (Actor|SetLifeSpan _returnvalue 5.0)
  (Utilities|Array|Add (Variables|Default|GetLevelsLoaded) _returnvalue))

(event EventBeginPlay
  (Utilities|Time|SetTimerbyEvent (delegate Custom|CustomEvent) 1.0 true))

(event EventTick
  (params (DeltaSeconds :type Float%20%28single-precision%29))
  (for _array_element (Variables|Default|GetLevelsLoaded)
    (Utilities|IsValid _array_element
      (:Is%20Valid
        (Transformation|AddActorWorldOffset _array_element (* DeltaSeconds (Variables|Default|GetVelocity)))))))

(fn ConstructionScript)