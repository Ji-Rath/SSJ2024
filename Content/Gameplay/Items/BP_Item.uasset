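; BP_Item is a world pickup actor that a player collects by overlapping it.
; The construction script sets its static mesh by synchronously loading the mesh referenced in its ItemInfo data.
; On overlap by a pawn with a PlayerController, it generates one item from ItemInfo and adds it to the InventoryComponent on the PlayerState.
; It then plays a 2D jingle and destroys itself.
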(event Collision|EventActorBeginOverlap
  (params (OtherActor :type Actor%20Object%20Reference))
  (bind _aspawn (Utilities|Casting|CastToPawn OtherActor))
  (if (Class|GameplayStatics|ObjectIsA (Pawn|GetController _aspawn) "/Script/Engine.PlayerController")
    (Class|InventoryComponent|AddtoInventory (Actor|GetComponentbyClass (Variables|/Script/Engine.Controller|GetPlayerState (Pawn|GetController _aspawn)) "/Script/InteractionSystem.InventoryComponent") (Class|InventoryComponent|GenerateItem :self (Actor|GetComponentbyClass (Variables|/Script/Engine.Controller|GetPlayerState (Pawn|GetController _aspawn)) "/Script/InteractionSystem.InventoryComponent") :ItemInfo (Variables|Default|GetItem%20Info)))
    (Audio|PlaySound2D "/Game/Sounds/Jingles/jingles_NES12.jingles_NES12" 1.0 1.0 0.0 0 0)
    (Actor|DestroyActor)))

(fn ConstructionScript
  (bind _item_info (Variables|Default|GetItem%20Info)
    (:then
      (bind _itemmesh (Variables|/Script/InteractionSystem.ItemInformation|GetItemMesh _item_info)
        (:then
          (bind _returnvalue (Utilities|LoadAssetBlocking _itemmesh))
          (bind _asstatic_mesh (Utilities|Casting|CastToStaticMesh _returnvalue))
          (Components|StaticMesh|SetStaticMesh (Variables|Default|GetStaticMesh) _asstatic_mesh))
        (:else)))
    (:else)))