(event Input|EnhancedActionEvents|EnhancedInputActionIA_Interact
  (params (ActionValue :type Boolean) (ElapsedSeconds :type Float%20%28double-precision%29) (TriggeredSeconds :type Float%20%28double-precision%29) (InputAction :type Input%20Action%20Object%20Reference :default "/Game/Input/IA_Interact.IA_Interact"))
  (:Started
    (Class|InteractorComponent|Interact (Variables|Default|GetAreaInteract))))

(event Input|EnhancedActionEvents|EnhancedInputActionIA_BuildMode
  (params (ActionValue :type Boolean) (ElapsedSeconds :type Float%20%28double-precision%29) (TriggeredSeconds :type Float%20%28double-precision%29) (InputAction :type Input%20Action%20Object%20Reference :default "/Game/Input/IA_BuildMode.IA_BuildMode"))
  (:Started
    (CallFunction|ToggleBuildMode)))

(event Input|EnhancedActionEvents|EnhancedInputActionIA_PrimaryAction
  (params (ActionValue :type Boolean) (ElapsedSeconds :type Float%20%28double-precision%29) (TriggeredSeconds :type Float%20%28double-precision%29) (InputAction :type Input%20Action%20Object%20Reference :default "/Game/Input/IA_PrimaryAction.IA_PrimaryAction"))
  (:Started
    (if (Variables|BuildMode|GetbBuildMode)
      (bind (_returnvalue _outhit) (CallFunction|GetMouseHit))
      (if _returnvalue
        (if (Class|GameplayStatics|ObjectIsA (.HitActor (Collision|BreakHitResult _outhit)) "/Game/Gameplay/BuildingBlocks/BP_BlockBase.BP_BlockBase_C")
          (Default|GrabComponent (Variables|Default|GetPhysicsSpringArm) (.HitComponent (Collision|BreakHitResult _outhit)))
          (Variables|BuildMode|SetbGrabbedBlock true)))))
  (:Completed
    (Variables|BuildMode|SetbGrabbedBlock false)
    (Default|ReleaseComponent (Variables|Default|GetPhysicsSpringArm))))

(event Input|EnhancedActionEvents|EnhancedInputActionIA_RotateItem
  (params (ActionValue :type Vector%202D%20Structure) (ElapsedSeconds :type Float%20%28double-precision%29) (TriggeredSeconds :type Float%20%28double-precision%29) (InputAction :type Input%20Action%20Object%20Reference :default "/Game/Input/IA_RotateItem.IA_RotateItem"))
  (bind _rotateitemmultiplier (Variables|BuildMode|GetRotateItemMultiplier))
  (bind _returnvalue (* ActionValue _rotateitemmultiplier))
  (bind (_x _y) (Math|Vector2D|BreakVector2D _returnvalue))
  (bind _attachedcomponent (Variables|/InteractionSystem/BPC_PhysicsGrab.BPC_PhysicsGrab_C|GetAttachedComponent (Variables|Default|GetPhysicsSpringArm))
    (:then
      (Class|PrimitiveComponent|AddForceatLocationLocal _attachedcomponent (Math|Vector|MakeVector 0.0 (* _y 1e+05) 0.0) (Math|Vector|MakeVector 1e+03 0.0 0.0) "None") ; Pitch
      (Class|PrimitiveComponent|AddForceatLocationLocal _attachedcomponent (Math|Vector|MakeVector 0.0 0.0 (* _x 1e+05)) (Math|Vector|MakeVector 0.0 1e+03 0.0) "None") ; Yaw
    )
    (:else)))

(event EventAsyncPhysicsTick
  (params (DeltaSeconds :type Float%20%28single-precision%29) (SimSeconds :type Float%20%28single-precision%29))
  (CallFunction|UpdateGrabTargetLocation))

(fn ConstructionScript)

(fn ToggleBuildMode
  (bind _output_get (Variables|BuildMode|SetbBuildMode (not (Variables|BuildMode|GetbBuildMode))))
  (if _output_get
    (Variables|BuildMode|SetOldSpringLen (Variables|/Script/Engine.SpringArmComponent|GetTargetArmLength (Variables|Default|GetSpringArm)))
    (Variables|/Script/Engine.SpringArmComponent|SetTargetArmLength (Variables|Default|GetSpringArm) (Variables|BuildMode|GetBuildModeSpringLen))
    (bind _hud (CallFunction|GetControlledHUD))
    (bind _mainui (Class|IGameHUD|GetMainUI(Message) _hud))
    (bind _returnvalue (Class|CommonActivatableWidgetContainerBase|AddWidget (Variables|/Game/UI/UI_Game.UI_Game_C|GetFullscreenQueue _mainui) "/Game/UI/Widgets/WBP_BuildMode.WBP_BuildMode_C"))
    (Variables|Default|SetBuildWidget _returnvalue)
    (bind _asplayer_controller (Utilities|Casting|CastToPlayerController (Pawn|GetController)))
    (Input|RemoveMappingContext (PlayerController|LocalPlayerSubsystems|GetEnhancedInputLocalPlayerSubsystem _asplayer_controller) "/Game/Input/IMC_Default.IMC_Default" "(bIgnoreAllPressedKeysUntilRelease=True,bForceImmediately=False,bNotifyUserSettings=False)")
    (Input|AddMappingContext (PlayerController|LocalPlayerSubsystems|GetEnhancedInputLocalPlayerSubsystem _asplayer_controller) "/Game/Input/IMC_BuildMode.IMC_BuildMode" 0 "(bIgnoreAllPressedKeysUntilRelease=True,bForceImmediately=False,bNotifyUserSettings=False)")
    (else
      (Variables|/Script/Engine.SpringArmComponent|SetTargetArmLength (Variables|Default|GetSpringArm) (Variables|BuildMode|GetOldSpringLen))
      (bind _buildwidget (Variables|Default|GetBuildWidget)
        (:then
          (Class|CommonActivatableWidget|DeactivateWidget _buildwidget)
          (bind _asplayer_controller_2 (Utilities|Casting|CastToPlayerController (Pawn|GetController)))
          (Input|RemoveMappingContext (PlayerController|LocalPlayerSubsystems|GetEnhancedInputLocalPlayerSubsystem _asplayer_controller_2) "/Game/Input/IMC_BuildMode.IMC_BuildMode" "(bIgnoreAllPressedKeysUntilRelease=True,bForceImmediately=False,bNotifyUserSettings=False)")
          (Input|AddMappingContext (PlayerController|LocalPlayerSubsystems|GetEnhancedInputLocalPlayerSubsystem _asplayer_controller_2) "/Game/Input/IMC_Default.IMC_Default" 0 "(bIgnoreAllPressedKeysUntilRelease=True,bForceImmediately=False,bNotifyUserSettings=False)"))
        (:else)))))

(fn GetControlledHUD
  (bind _asplayer_controller (Utilities|Casting|CastToPlayerController (Pawn|GetController))
    (:then
      (return (HUD|GetHUD _asplayer_controller)))
    (:CastFailed
      (return 0))))

(fn GetMouseHit
  (bind _returnvalue (Game|GetPlayerController 0))
  (bind (_worldlocation _worlddirection) (Game|Player|ConvertMouseLocationToWorldSpace _returnvalue))
  (Utilities|FlowControl|Sequence
    (:then_0
      (bind _attachedcomponent (Variables|/InteractionSystem/BPC_PhysicsGrab.BPC_PhysicsGrab_C|GetAttachedComponent (Variables|Default|GetPhysicsSpringArm))
        (:then
          (Utilities|Array|Add (LocalVariables|GetIgnoreArray) (Components|GetOwner _attachedcomponent)))
        (:else)))
    (:then_1
      (bind (_outhit _returnvalue_2) (Collision|LineTraceByChannel _worldlocation (+ _worldlocation (* _worlddirection (Variables|BuildMode|GetSelectBlockTraceLen))) "TraceTypeQuery1" false (LocalVariables|GetIgnoreArray) "None"))
      (return _returnvalue_2 _outhit))))

(fn UpdateGrabTargetLocation
  (Variables|/InteractionSystem/BPC_PhysicsGrab.BPC_PhysicsGrab_C|GetAttachedComponent (Variables|Default|GetPhysicsSpringArm)
    (:then
      (bind (_returnvalue _outhit) (CallFunction|GetMouseHit))
      (Default|SetTargetLocation (Variables|Default|GetPhysicsSpringArm) (Math|Vector|SelectVector (.Intersection (Class|KismetMathLibrary|LinePlaneIntersection (.TraceStart (Collision|BreakHitResult _outhit)) (Math|Vector|SelectVector (.Location (Collision|BreakHitResult _outhit)) (.TraceEnd (Collision|BreakHitResult _outhit)) _returnvalue) (Class|KismetMathLibrary|MakePlanefromPointandNormal (Transformation|GetActorLocation) "1.000000,0.000000,0.000000"))) (Math|Vector|SelectVector (.Location (Collision|BreakHitResult _outhit)) (.TraceEnd (Collision|BreakHitResult _outhit)) _returnvalue) (.ReturnValue (Class|KismetMathLibrary|LinePlaneIntersection (.TraceStart (Collision|BreakHitResult _outhit)) (Math|Vector|SelectVector (.Location (Collision|BreakHitResult _outhit)) (.TraceEnd (Collision|BreakHitResult _outhit)) _returnvalue) (Class|KismetMathLibrary|MakePlanefromPointandNormal (Transformation|GetActorLocation) "1.000000,0.000000,0.000000"))))))
    (:else)))