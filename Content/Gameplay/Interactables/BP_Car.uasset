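; BP_Car is a single-use interactable car that acts as the game's win trigger.
; On interact by a pawn, it tries to complete the place-parts task of the car-fix SUQS quest, assuming reaching that task means the player has the parts.
; Success adds the win-game widget to the main UI's fullscreen stack; otherwise it plays the car monologue through the HUD.
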(event EventInteract
  (params (Interactor :type Actor%20Object%20Reference) (Component :type Scene%20Component%20Object%20Reference))
  (bind _aspawn (Utilities|Casting|CastToPawn Interactor))
  (bind _progression (Class|ISUQSProgression|GetSUQSProgression(Message) (Game|GetGameInstance)))
  (bind _returnvalue (Class|SuqsProgression|CompleteTask _progression "Q_CarFix" "T_PlacePartsInCar")) ; We make the assumption that if the player reached this task, they have the parts and can fix the car
  (if _returnvalue
    (bind _asplayer_controller (Utilities|Casting|CastToPlayerController (Pawn|GetController _aspawn)))
    (bind _mainui (Class|IGameHUD|GetMainUI(Message) (HUD|GetHUD _asplayer_controller)))
    (Class|CommonActivatableWidgetContainerBase|AddWidget (Variables|/Game/UI/UI_Game.UI_Game_C|GetFullscreenStack _mainui) "/Game/UI/Widgets/WBP_WinGame.WBP_WinGame_C")
    (else
      (bind _returnvalue_2 (Class|DlgManager|StartMonologue "/Game/Gameplay/Dialogue/DLG_Car.DLG_Car" Interactor))
      (Class|IGameHUD|DisplayDialogue(Message) (HUD|GetHUD (Game|GetPlayerController 0)) _returnvalue_2))))

(fn ConstructionScript)

(fn CanInteract
  (params (Interactor :type Actor%20Object%20Reference) (Component :type Scene%20Component%20Object%20Reference))
  (return true))

(fn GetInteractType
  (return "SingleUse"))

(fn GetName
  (params (Component :type Scene%20Component%20Object%20Reference))
  (return ""))