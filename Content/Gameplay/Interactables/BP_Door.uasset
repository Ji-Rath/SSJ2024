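; BP_Door is a single-use interactable door that plays an opening animation and moves the player to another level.
; Interact accepts only player-controlled pawns, fires once, then after a short delay asks BP_LevelManager to load LevelToLoad with TargetSpawnTag.
; CanInteract can optionally gate the door on a SUQS task, always looked up in the hardcoded Q_CarFix quest.
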(event EventBeginPlay)

(event Collision|EventActorBeginOverlap
  (params (OtherActor :type Actor%20Object%20Reference)))

(event EventTick
  (params (DeltaSeconds :type Float%20%28single-precision%29)))

(event EventInteract
  (params (Interactor :type Actor%20Object%20Reference) (Component :type Scene%20Component%20Object%20Reference))
  (bind _aspawn (Utilities|Casting|CastToPawn Interactor))
  (Utilities|Casting|CastToPlayerController (Pawn|GetController _aspawn))
  (Utilities|FlowControl|DoOnce false
    (:Completed
      (Components|Animation|PlayAnimation (Variables|Default|GetSkeletalMesh) (Variables|Door|Visual|GetDoorOpenAnimation) false)
      (Utilities|FlowControl|Delay 0.5)
      (bind _returnvalue (Actor|GetActorOfClass "/Game/Gameplay/LevelLoading/BP_LevelManager.BP_LevelManager_C"))
      (Default|LoadLevel _returnvalue (Variables|Door|GetLevelToLoad) (Variables|Door|GetTargetSpawnTag)))))

(fn ConstructionScript)

(fn CanInteract
  (params (Interactor :type Actor%20Object%20Reference) (Component :type Scene%20Component%20Object%20Reference))
  (if (Variables|Door|Condition|GetbRequireTaskCompleted)
    (bind _progression (Class|ISUQSProgression|GetSUQSProgression(Message) (Game|GetGameInstance)))
    (return (Class|SuqsProgression|IsTaskCompleted _progression "Q_CarFix" (Variables|Door|Condition|GetTaskToComplete)))
    (else
      (return true))))

(fn GetInteractType
  (return "SingleUse"))

(fn GetName
  (params (Component :type Scene%20Component%20Object%20Reference))
  (return ""))