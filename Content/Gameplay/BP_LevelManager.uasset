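; Level manager that swaps one streamed level instance at a time and moves the player to a tagged spawn point in it.
; LoadLevel stores the spawn tag, unloads the current instance, loads the new one from a soft reference and binds to its loaded event, printing an error on failure.
; LevelLoaded broadcasts OnLevelLoad, then teleports player pawn 0 to the location of the first PlayerStart with that tag.
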(fn ConstructionScript)

(fn LoadLevel
  (params (Level :type World%20Soft%20Object%20Reference) (Tag :type Name :default "DefaultSpawn"))
  (Variables|Default|SetSpawnTag Tag)
  (bind _currentlyloadedlevel (Variables|Default|GetCurrentlyLoadedLevel)
    (:then
      (Class|LevelInstanceInterface|UnloadLevelInstance(Message) _currentlyloadedlevel)
      (Variables|Default|SetCurrentlyLoadedLevel 0))
    (:else
      _))
  (bind (_boutsuccess _returnvalue) (Class|LevelStreamingDynamic|LoadLevelInstancebySoftObjectPtr Level "0, 0, 0" "0, 0, 0" "" "/Script/Engine.LevelStreamingDynamic" false))
  (if _boutsuccess
    (bind _output_get (Variables|Default|SetCurrentlyLoadedLevel _returnvalue))
    (EventDispatchers|BindEventtoOnLevelLoaded _output_get (EventDispatchers|CreateEvent :!event LevelLoaded))
    (else
      (Development|PrintString "Error: Unable to load level!"))))

(fn LevelLoaded
  (Default|CallOnLevelLoad (Variables|Default|GetCurrentlyLoadedLevel))
  (bind _outactors (Actor|GetAllActorsOfClasswithTag "/Script/Engine.PlayerStart" (Variables|Default|GetSpawnTag)))
  (if (Utilities|Array|IsNotEmpty _outactors)
    (Transformation|SetActorLocation (Game|Player|GetPlayerPawn 0) (Transformation|GetActorLocation (Utilities|Array|Get(acopy) _outactors)) false true)))