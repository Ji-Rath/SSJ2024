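; Level manager that swaps streamed level instances and places the player at a tagged spawn point.
; LoadLevel stores the spawn tag, requests unload of the current instance and loads the new one from a soft reference.
; On load completion it broadcasts OnLevelLoad and flags a pending reposition.
; AddLocationPoint collects points and teleports player 0 to the first matching one registered while that flag is set.
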(fn ConstructionScript)

(fn LoadLevel
  (params (Level :type World%20Soft%20Object%20Reference) (Tag :type Name :default "DefaultSpawn"))
  (Variables|Default|SetSpawnTag Tag)
  (bind _currentlyloadedlevel (Variables|Default|GetCurrentlyLoadedLevel)
    (:then
      (Class|LevelStreaming|SetIsRequestingUnloadandRemoval _currentlyloadedlevel true)
      (Variables|Default|SetCurrentlyLoadedLevel 0))
    (:else
      _))
  (bind (_boutsuccess _returnvalue) (Class|LevelStreamingDynamic|LoadLevelInstancebySoftObjectPtr Level "0, 0, 0" "0, 0, 0" "" "/Script/Engine.LevelStreamingDynamic" false))
  (if _boutsuccess
    (bind _output_get (Variables|Default|SetCurrentlyLoadedLevel _returnvalue))
    (EventDispatchers|BindEventtoOnLevelLoaded _output_get (EventDispatchers|CreateEvent :!event LevelLoaded))
    (else
      (Development|PrintString "Error: Unable to load level!"))))

(fn LevelLoaded
  (Default|CallOnLevelLoad (Variables|Default|GetCurrentlyLoadedLevel))
  (Variables|Default|SetbNeedsNewPosition true))

(fn AddLocationPoint
  (params (LocationPoint :type BP%20Location%20Point%20Object%20Reference%20%28by%20ref%29))
  (Utilities|Array|AddUnique (Variables|Default|GetLocationPoints) LocationPoint)
  (if (and (Actor|ActorHasTag LocationPoint (Variables|Default|GetSpawnTag)) (Variables|Default|GetbNeedsNewPosition))
    (Variables|Default|SetbNeedsNewPosition false)
    (Transformation|SetActorLocation (Game|Player|GetPlayerPawn 0) (Transformation|GetActorLocation LocationPoint) false true)))