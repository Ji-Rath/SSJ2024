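; BP_BlockCameraCapture is an editor-side tool actor that renders display textures for the block classes in BlockList.
; RenderBlocks swaps each class into a ChildActor, disables physics on its primitives, and captures it alone through a show-only SceneCaptureComponent2D.
; For BP_BlockBase blocks, the editor-only render target conversion then writes the capture into that block's TextureDisplay texture.
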(event Custom|RenderBlocks
  (bind _scenecapturecomponent2d (Variables|Default|GetSceneCaptureComponent2D))
  (for _array_element (Variables|Default|GetBlockList)
    (ChildActorComponent|SetChildActorClass (Variables|Default|GetChildActor) (Utilities|ResolveSoftReference _array_element))
    (for _array_element_2 (Actor|GetComponentsByClass (Variables|/Script/Engine.ChildActorComponent|GetChildActor (Variables|Default|GetChildActor)) "/Script/Engine.PrimitiveComponent")
      (Physics|SetSimulatePhysics _array_element_2 false))
    (Rendering|SceneCapture|ShowOnlyActorComponents (Variables|Default|GetSceneCaptureComponent2D) (Variables|/Script/Engine.ChildActorComponent|GetChildActor (Variables|Default|GetChildActor)) true)
    (Rendering|SceneCapture|CaptureScene _scenecapturecomponent2d :!class /Script/Engine.SceneCaptureComponent2D)
    (bind _asbp_block_base (Utilities|Casting|CastToBP_BlockBase (Variables|/Script/Engine.ChildActorComponent|GetChildActor (Variables|Default|GetChildActor))))
    (EditorScripting|Rendering|ConvertRenderTargettoTexture2DEditorOnly (Variables|/Script/Engine.SceneCaptureComponent2D|GetTextureTarget _scenecapturecomponent2d) (Utilities|ResolveSoftReference (Variables|/Game/Gameplay/BuildingBlocks/BP_BlockBase.BP_BlockBase_C|GetTextureDisplay _asbp_block_base)))))

(fn ConstructionScript)