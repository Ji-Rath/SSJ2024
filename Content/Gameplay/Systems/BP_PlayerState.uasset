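; Player state that links item pickups to progress in the car repair quest.
; When its Inventory component reports an added item, a branch chain compares the item's data asset against the fuse, oil and wheel.
; A match completes the corresponding Q_CarFix task through the SUQS progression object obtained from the Game Instance.
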(event OnItemAdd(Inventory)
  (params (Item :type Inventory%20Contents%20Structure%20%28by%20ref%29))
  (bind _iteminformation (Utilities|Struct|BreakInventoryContents Item))
  (bind _progression (Class|ISUQSProgression|GetSUQSProgression(Message) (Game|GetGameInstance)))
  (if (== _iteminformation "/Game/Gameplay/Items/DA_Fuse.DA_Fuse")
    (Class|SuqsProgression|CompleteTask _progression "Q_CarFix" "T_GetFuse")
    (elif (== _iteminformation "/Game/Gameplay/Items/DA_Oil.DA_Oil")
      (Class|SuqsProgression|CompleteTask _progression "Q_CarFix" "T_GetOil")
      (elif (== _iteminformation "/Game/Gameplay/Items/DA_Wheel.DA_Wheel")
        (Class|SuqsProgression|CompleteTask _progression "Q_CarFix" "T_GetWheel")))))

(event EventBeginPlay)

(event EventTick
  (params (DeltaSeconds :type Float%20%28single-precision%29)))

(fn ConstructionScript)