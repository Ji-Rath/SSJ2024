(event Input|EnhancedActionEvents|EnhancedInputActionIA_Interact
  (params (ActionValue :type Boolean) (ElapsedSeconds :type Float%20%28double-precision%29) (TriggeredSeconds :type Float%20%28double-precision%29) (InputAction :type Input%20Action%20Object%20Reference :default "/Game/Input/Actions/IA_Interact.IA_Interact"))
  (:Started
    (Class|InteractorComponent|Interact (Variables|Default|GetAreaInteract))))

(event Game|Damage|EventAnyDamage
  (params (Damage :type Float%20%28single-precision%29) (DamageType :type Damage%20Type%20Object%20Reference) (InstigatedBy :type Controller%20Object%20Reference) (DamageCauser :type Actor%20Object%20Reference))
  (bind _returnvalue (Actor|GetActorOfClass "/Game/Gameplay/LevelLoading/BP_LocationPoint.BP_LocationPoint_C"))
  (bind _returnvalue_2 (Game|SpawnActorfromClass "BP_Player_C" (Math|Conversions|ToTransform(Vector) (Transformation|GetActorLocation _returnvalue)) "Undefined" "MultiplyWithRoot" 0 0))
  (Pawn|Possess (Game|GetPlayerController 0) _returnvalue_2)
  (Actor|DestroyActor))

(event Input|EnhancedActionEvents|EnhancedInputActionIA_BuildMode
  (params (ActionValue :type Boolean) (ElapsedSeconds :type Float%20%28double-precision%29) (TriggeredSeconds :type Float%20%28double-precision%29) (InputAction :type Input%20Action%20Object%20Reference :default "/Game/Input/Actions/IA_BuildMode.IA_BuildMode"))
  (:Started
    (CallFunction|ToggleBuildMode)))

(event Input|EnhancedActionEvents|EnhancedInputActionIA_PrimaryAction
  (params (ActionValue :type Boolean) (ElapsedSeconds :type Float%20%28double-precision%29) (TriggeredSeconds :type Float%20%28double-precision%29) (InputAction :type Input%20Action%20Object%20Reference :default "/Game/Input/Actions/IA_PrimaryAction.IA_PrimaryAction"))
  (:Started
    (if (Variables|BuildMode|GetbBuildMode)
      (bind (_returnvalue _outhit) (CallFunction|GetMouseHit))
      (if _returnvalue
        (if (Class|GameplayStatics|ObjectIsA (.HitActor (Collision|BreakHitResult _outhit)) "/Game/Gameplay/BuildingBlocks/BP_BlockBase.BP_BlockBase_C")
          (Default|GrabComponent (Variables|Default|GetPhysicsSpringArm) (.HitComponent (Collision|BreakHitResult _outhit)))
          (Variables|BuildMode|SetbGrabbedBlock true)
          (else
            (Game|Damage|ApplyDamage (.HitActor (Collision|BreakHitResult _outhit)) 5.0 0 0))))))
  (:Completed
    (Variables|BuildMode|SetbGrabbedBlock false)
    (Default|ReleaseComponent (Variables|Default|GetPhysicsSpringArm))))

(event Input|EnhancedActionEvents|EnhancedInputActionIA_RotateItem
  (params (ActionValue :type Vector%202D%20Structure) (ElapsedSeconds :type Float%20%28double-precision%29) (TriggeredSeconds :type Float%20%28double-precision%29) (InputAction :type Input%20Action%20Object%20Reference :default "/Game/Input/Actions/IA_RotateItem.IA_RotateItem"))
  (bind _rotateforce (Variables|Default|GetRotateForce))
  (bind _rotateitemmultiplier (Variables|BuildMode|GetRotateItemMultiplier))
  (bind _returnvalue (* ActionValue _rotateitemmultiplier))
  (bind (_x _y) (Math|Vector2D|BreakVector2D _returnvalue))
  (bind _attachedcomponent (Variables|/InteractionSystem/BPC_PhysicsGrab.BPC_PhysicsGrab_C|GetAttachedComponent (Variables|Default|GetPhysicsSpringArm))
    (:then
      (Class|PrimitiveComponent|AddForceatLocationLocal _attachedcomponent (Math|Vector|MakeVector 0.0 (* _y _rotateforce) 0.0) (Math|Vector|MakeVector 1e+03 0.0 0.0) "None") ; Pitch
      (Class|PrimitiveComponent|AddForceatLocationLocal _attachedcomponent (Math|Vector|MakeVector 0.0 0.0 (* _x _rotateforce)) (Math|Vector|MakeVector 0.0 1e+03 0.0) "None") ; Yaw
    )
    (:else)))

(event EventAsyncPhysicsTick
  (params (DeltaSeconds :type Float%20%28single-precision%29) (SimSeconds :type Float%20%28single-precision%29))
  (CallFunction|UpdateGrabTargetLocation))

(fn ConstructionScript)

(fn ToggleBuildMode
  (bind _output_get (Variables|BuildMode|SetbBuildMode (not (Variables|BuildMode|GetbBuildMode))))
  (if _output_get
    (Variables|BuildMode|SetOldSpringLen (Variables|/Script/Engine.SpringArmComponent|GetTargetArmLength (Variables|Default|GetSpringArm)))
    (Variables|/Script/Engine.SpringArmComponent|SetTargetArmLength (Variables|Default|GetSpringArm) (Variables|BuildMode|GetBuildModeSpringLen))
    (bind _hud (CallFunction|GetControlledHUD))
    (bind _mainui (Class|IGameHUD|GetMainUI(Message) _hud))
    (bind _returnvalue (Class|CommonActivatableWidgetContainerBase|AddWidget (Variables|/Game/UI/UI_Game.UI_Game_C|GetFullscreenQueue _mainui) "/Game/UI/Widgets/ConstructMode/WBP_BuildMode.WBP_BuildMode_C"))
    (Utilities|Array|Add (Variables|Default|GetBuildWidget) _returnvalue)
    (bind _returnvalue_2 (Class|CommonActivatableWidgetContainerBase|AddWidget (Variables|/Game/UI/UI_Game.UI_Game_C|GetBottomQueue _mainui) "/Game/UI/Widgets/ConstructMode/WBP_CraftingBlocks.WBP_CraftingBlocks_C"))
    (Utilities|Array|Add (Variables|Default|GetBuildWidget) _returnvalue_2)
    (bind _asplayer_controller (Utilities|Casting|CastToPlayerController (Pawn|GetController)))
    (Input|RemoveMappingContext (PlayerController|LocalPlayerSubsystems|GetEnhancedInputLocalPlayerSubsystem _asplayer_controller) "/Game/Input/IMC_Default.IMC_Default" "(bIgnoreAllPressedKeysUntilRelease=True,bForceImmediately=False,bNotifyUserSettings=False)")
    (Input|AddMappingContext (PlayerController|LocalPlayerSubsystems|GetEnhancedInputLocalPlayerSubsystem _asplayer_controller) "/Game/Input/IMC_BuildMode.IMC_BuildMode" 0 "(bIgnoreAllPressedKeysUntilRelease=True,bForceImmediately=False,bNotifyUserSettings=False)")
    (else
      (Variables|/Script/Engine.SpringArmComponent|SetTargetArmLength (Variables|Default|GetSpringArm) (Variables|BuildMode|GetOldSpringLen))
      (for _array_element (Variables|Default|GetBuildWidget)
        (Class|CommonActivatableWidget|DeactivateWidget _array_element))
      (bind _asplayer_controller_2 (Utilities|Casting|CastToPlayerController (Pawn|GetController)))
      (Input|RemoveMappingContext (PlayerController|LocalPlayerSubsystems|GetEnhancedInputLocalPlayerSubsystem _asplayer_controller_2) "/Game/Input/IMC_BuildMode.IMC_BuildMode" "(bIgnoreAllPressedKeysUntilRelease=True,bForceImmediately=False,bNotifyUserSettings=False)")
      (Input|AddMappingContext (PlayerController|LocalPlayerSubsystems|GetEnhancedInputLocalPlayerSubsystem _asplayer_controller_2) "/Game/Input/IMC_Default.IMC_Default" 0 "(bIgnoreAllPressedKeysUntilRelease=True,bForceImmediately=False,bNotifyUserSettings=False)"))))

(fn GetControlledHUD
  (bind _asplayer_controller (Utilities|Casting|CastToPlayerController (Pawn|GetController))
    (:then
      (return (HUD|GetHUD _asplayer_controller)))
    (:CastFailed
      (return 0))))

(fn GetMouseHit
  (bind _returnvalue (Game|GetPlayerController 0))
  (bind (_worldlocation _worlddirection) (Game|Player|ConvertMouseLocationToWorldSpace _returnvalue))
  (Utilities|FlowControl|Sequence
    (:then_0
      (bind _attachedcomponent (Variables|/InteractionSystem/BPC_PhysicsGrab.BPC_PhysicsGrab_C|GetAttachedComponent (Variables|Default|GetPhysicsSpringArm))
        (:then
          (Utilities|Array|Add (LocalVariables|GetIgnoreArray) (Components|GetOwner _attachedcomponent)))
        (:else)))
    (:then_1
      (bind (_outhit _returnvalue_2) (Collision|LineTraceByChannel _worldlocation (+ _worldlocation (* _worlddirection (Variables|BuildMode|GetSelectBlockTraceLen))) "TraceTypeQuery1" false (LocalVariables|GetIgnoreArray) "None"))
      (return _returnvalue_2 _outhit))))

(fn UpdateGrabTargetLocation
  (Variables|/InteractionSystem/BPC_PhysicsGrab.BPC_PhysicsGrab_C|GetAttachedComponent (Variables|Default|GetPhysicsSpringArm)
    (:then
      (bind (_returnvalue _outhit) (CallFunction|GetMouseHit))
      (Default|SetTargetLocation (Variables|Default|GetPhysicsSpringArm) (Math|Vector|SelectVector (.Intersection (Class|KismetMathLibrary|LinePlaneIntersection (.TraceStart (Collision|BreakHitResult _outhit)) (Math|Vector|SelectVector (.Location (Collision|BreakHitResult _outhit)) (.TraceEnd (Collision|BreakHitResult _outhit)) _returnvalue) (Class|KismetMathLibrary|MakePlanefromPointandNormal (Transformation|GetActorLocation) "1.000000,0.000000,0.000000"))) (Math|Vector|SelectVector (.Location (Collision|BreakHitResult _outhit)) (.TraceEnd (Collision|BreakHitResult _outhit)) _returnvalue) (.ReturnValue (Class|KismetMathLibrary|LinePlaneIntersection (.TraceStart (Collision|BreakHitResult _outhit)) (Math|Vector|SelectVector (.Location (Collision|BreakHitResult _outhit)) (.TraceEnd (Collision|BreakHitResult _outhit)) _returnvalue) (Class|KismetMathLibrary|MakePlanefromPointandNormal (Transformation|GetActorLocation) "1.000000,0.000000,0.000000"))))))
    (:else)))

(fn CheckCondition
  (params (Context :type Dlg%20Context%20Object%20Reference) (ConditionName :type Name :default "None"))
  (return false))

(fn GetBoolValue
  (params (ValueName :type Name :default "None"))
  (return false))

(fn GetFloatValue
  (params (ValueName :type Name :default "None"))
  (return 0.0))

(fn GetIntValue
  (params (ValueName :type Name :default "None"))
  (return 0))

(fn GetNameValue
  (params (ValueName :type Name :default "None"))
  (return "None"))

(fn GetParticipantDisplayName
  (params (ActiveSpeaker :type Name :default "None"))
  (return ""))

(fn GetParticipantGender
  (return "Masculine"))

(fn GetParticipantIcon
  (params (ActiveSpeaker :type Name :default "None") (ActiveSpeakerState :type Name :default "None"))
  (return 0))

(fn GetParticipantName
  (return "Player"))

(fn ModifyBoolValue
  (params (ValueName :type Name :default "None") (bNewValue :type Boolean))
  (return false))

(fn ModifyFloatValue
  (params (ValueName :type Name :default "None") (bDelta :type Boolean) (Value :type Float%20%28single-precision%29))
  (return false))

(fn ModifyIntValue
  (params (ValueName :type Name :default "None") (bDelta :type Boolean) (Value :type Integer))
  (return false))

(fn ModifyNameValue
  (params (ValueName :type Name :default "None") (NameValue :type Name :default "None"))
  (return false))

(fn OnDialogueEvent
  (params (Context :type Dlg%20Context%20Object%20Reference) (EventName :type Name :default "None"))
  (return false))