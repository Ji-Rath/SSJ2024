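; BP_Spring is a spring building block that launches whatever hits it, limited by a cooldown.
; On a hit after the cooldown, it queues a fixed jump impulse as an instant movement effect on the other actor's MoverComponent, if present.
; It also fires a RadialForce impulse, whether or not a Mover was found, and records the hit time.
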(event Collision|EventHit
  (params (MyComp :type Primitive%20Component%20Object%20Reference) (Other :type Actor%20Object%20Reference) (OtherComp :type Primitive%20Component%20Object%20Reference) (bSelfMoved :type Boolean) (HitLocation :type Vector :default "0, 0, 0") (HitNormal :type Vector :default "0, 0, 0") (NormalImpulse :type Vector :default "0, 0, 0") (Hit :type Hit%20Result%20Structure%20%28by%20ref%29))
  (bind _returnvalue (Actor|GetComponentbyClass Other "/Script/Mover.MoverComponent"))
  (if (> (Utilities|Time|GetTimeSeconds) (+ (Variables|Default|GetLastHit) (Variables|Default|GetSpringCooldown)))
    (Utilities|FlowControl|Sequence
      (:then_0
        (Utilities|IsValid _returnvalue
          (:Is%20Valid
            (Class|MoverComponent|QueueInstantMovementEffect _returnvalue (Utilities|Struct|MakeJumpImpulseEffect 1e+03)))))
      (:then_1
        (Class|RadialForceComponent|FireImpulse (Variables|Default|GetRadialForce))
        (Variables|Default|SetLastHit (Utilities|Time|GetTimeSeconds))))))

(fn ConstructionScript
  (|CallParentFunction))