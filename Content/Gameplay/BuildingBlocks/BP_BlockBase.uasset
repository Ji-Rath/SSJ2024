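; BP_BlockBase is a building block actor that handles falling into a kill Z volume.
; When ShouldRespawn is set, BeginPlay caches the static mesh's world transform.
; On overlap with a KillZVolume, a respawning block moves its mesh back to that transform and zeroes its linear velocity, while any other block destroys itself.
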(event EventBeginPlay
  (if (Variables|Default|GetbShouldRespawn)
    (Variables|Default|SetOriginalTransform (Transformation|GetWorldTransform (Variables|Default|GetStaticMesh)))))

(event Collision|EventActorBeginOverlap
  (params (OtherActor :type Actor%20Object%20Reference))
  (if (Class|GameplayStatics|ObjectIsA OtherActor "/Script/Engine.KillZVolume")
    (if (Variables|Default|GetbShouldRespawn)
      (Transformation|SetWorldTransform (Variables|Default|GetStaticMesh) (Variables|Default|GetOriginalTransform) false false)
      (Physics|SetPhysicsLinearVelocity (Variables|Default|GetStaticMesh) "0, 0, 0" false "None")
      (else
        (Actor|DestroyActor)))))

(fn ConstructionScript)